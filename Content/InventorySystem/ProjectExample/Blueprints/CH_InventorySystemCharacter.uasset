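; Example first-person character for the inventory system, wiring player input to an InventoryManager fetched on BeginPlay.
; Tab handlers toggle inventory and crafting display, flipping IsBeingControlled, which gates item use.
; OpenChest line-traces for a BP_StorageChest, caching it to close later and toggling the inventory alongside.
; Number keys and per-tick scroll polling select hotbar slots, SlotUpdate refreshes the selection, and drop inputs discard one item or the whole stack.
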(event EventBeginPlay
  ;[1 1 1] Inventory System code
  ;;[1 1 1] Get & Set the inventory manager
  (bind _inventorymanagercomponent (CallFunction|GetInventoryManager self))
  (Variables|Default|SetInventoryManager _inventorymanagercomponent))

(event Input|ActionEvents|InputActionOpenChest
  (params (Key :type Key%20Structure :default "None"))
  (bind _firstpersoncamera (Variables|MyCharacter|GetFirstPersonCamera))
  (bind _returnvalue (Transformation|GetWorldLocation _firstpersoncamera))
  ;[1 0.191 0.9392] Comment
  (:Pressed
    ;;[1 1 1] Is there a chest that the user has currently opened?
    (Utilities|IsValid (Variables|Default|GetCurrentlyOpenChest)
      (:Is%20Valid
        ;;[1 1 1] Close the chest by toggling it, and then setting the reference to none/null (so it won't think it is still open)
        (Default|ToggleChest (Variables|Default|GetCurrentlyOpenChest))
        (Variables|Default|SetCurrentlyOpenChest 0)
        (Default|ToggleInventoryOpen (Variables|Default|GetInventoryManager))
        (Variables|Default|SetIsBeingControlled? (not (Variables|Default|GetIsBeingControlled?))))
      (:Is%20Not%20Valid
        ;;[1 1 1] Open the chest by toggling it
        (bind _outhit (Collision|LineTraceByChannel _returnvalue (+ (* (Math|Vector|GetForwardVector _firstpersoncamera) (Variables|Default|GetChestOpenReach)) _returnvalue) "TraceTypeQuery1" false 0 "None"))
        (bind _asbp_storage_chest (Utilities|Casting|CastToBP_StorageChest (.HitActor (Collision|BreakHitResult _outhit))))
        (Default|ToggleChest _asbp_storage_chest)
        ;;;[1 1 1] Set the reference so we can later close this one
        (Variables|Default|SetCurrentlyOpenChest _asbp_storage_chest)
        (Default|ToggleInventoryOpen (Variables|Default|GetInventoryManager))
        (Variables|Default|SetIsBeingControlled? (not (Variables|Default|GetIsBeingControlled?)))))))

(event Input|ActionEvents|InputActionUseItem
  (params (Key :type Key%20Structure :default "None"))
  ;[1 1 1] Inventory System code
  ;;[1 1 1] Code for using an item in the selected hotbar slot (use RMB to use an item)
  (:Pressed
    (if (Variables|Default|GetIsBeingControlled?)
      (Default|DoUseItem (Variables|Default|GetInventoryManager)))))

(event Input|KeyboardEvents|Tab
  (params (Key :type Key%20Structure :default "None"))
  ;[1 1 1] Inventory System code
  ;;[1 1 1] Toggle if the inventory is open or not!
  (:Pressed
    (Default|ToggleInventoryOpen (Variables|Default|GetInventoryManager))
    ;;[1 1 1] Gain and Loose control over the character. In  here to save a cast!
    (Variables|Default|SetIsBeingControlled? (not (Variables|Default|GetIsBeingControlled?)))))

(event Input|KeyboardEvents|Tab
  (params (Key :type Key%20Structure :default "None"))
  ;[1 1 1] Inventory System code
  (:Pressed
    (Default|ToggleCraftingDisplayOpen (Variables|Default|GetInventoryManager))
    (Variables|Default|SetIsBeingControlled? (not (Variables|Default|GetIsBeingControlled?)))))

(event Custom|DoMouseScrollWheelHotbarUpdate
  (bind _returnvalue (Class|Actor|GetInputAxisKeyValue))
  (bind _inventorymanager (Variables|Default|GetInventoryManager))
  (bind _returnvalue_2 (Math|Float|Truncate _returnvalue))
  (bind _hotbarwidget (Variables|/Game/InventorySystem/Blueprints/BP_InventoryManagerComponent.BP_InventoryManagerComponent_C|GetHotbarWidget _inventorymanager))
  ;[1 1 1] The hotbar controls to operate everything to do with the hotbar!!!
  ;;[1 1 1] Do the scrollwheel for hotbar slots!
  ;;;[1 1 1] Check if the user scrolled
  (if (not (== _returnvalue_2 0))
    (bind _newparam (Default|SetSelectedSlot _hotbarwidget (+ (Variables|/Game/InventorySystem/UMG/WBP_HotbarWidget.WBP_HotbarWidget_C|GetSelectedSlotID _hotbarwidget) _returnvalue_2)))
    (Development|PrintString (Utilities|String|EnumtoString _newparam))))

(event Custom|SlotUpdate
  (params (Compare :type Integer) (Compare2 :type Integer))
  (bind _inventorymanager (Variables|Default|GetInventoryManager))
  (bind _hotbarwidget (Variables|/Game/InventorySystem/Blueprints/BP_InventoryManagerComponent.BP_InventoryManagerComponent_C|GetHotbarWidget _inventorymanager))
  (bind _selectedslotid (Variables|/Game/InventorySystem/UMG/WBP_HotbarWidget.WBP_HotbarWidget_C|GetSelectedSlotID _hotbarwidget))
  (if (or (== Compare _selectedslotid) (== Compare2 _selectedslotid))
    (bind _newparam (Default|SetSelectedSlot _hotbarwidget _selectedslotid))
    (Development|PrintString (Utilities|String|EnumtoString _newparam))))

(event EventTick
  (params (DeltaSeconds :type Float%20%28single-precision%29))
  ;[1 1 1] The hotbar controls to operate everything to do with the hotbar!!!
  ;;[1 1 1] Check for scrollwheel action and process it if needed!
  (CallFunction|DoMouseScrollWheelHotbarUpdate))

(event Input|ActionEvents|InputActionDropAllItems
  (params (Key :type Key%20Structure :default "None"))
  (bind _inventorymanager (Variables|Default|GetInventoryManager))
  (bind _hotbarwidget (Variables|/Game/InventorySystem/Blueprints/BP_InventoryManagerComponent.BP_InventoryManagerComponent_C|GetHotbarWidget _inventorymanager))
  (bind _selectedslotid (Variables|/Game/InventorySystem/UMG/WBP_HotbarWidget.WBP_HotbarWidget_C|GetSelectedSlotID _hotbarwidget))
  (bind _hotbarslots (Variables|/Game/InventorySystem/UMG/WBP_HotbarWidget.WBP_HotbarWidget_C|GetHotbarSlots _hotbarwidget))
  (bind _output (Utilities|Array|Get(acopy) _hotbarslots _selectedslotid))
  ;[1 1 1] The hotbar controls to operate everything to do with the hotbar!!!
  ;;[1 1 1] DoItemDropping
  ;;;[1 1 1] Drop all remaining items
  (:Pressed
    (Utilities|IsValid _output
      (:Is%20Valid
        (Default|DropItematIndex _inventorymanager (Variables|/Game/InventorySystem/UMG/WBP_HotbarSlot.WBP_HotbarSlot_C|GetSlotID _output) -1)))))

(event Input|ActionEvents|InputActionDropSingleItem
  (params (Key :type Key%20Structure :default "None"))
  (bind _inventorymanager (Variables|Default|GetInventoryManager))
  (bind _hotbarwidget (Variables|/Game/InventorySystem/Blueprints/BP_InventoryManagerComponent.BP_InventoryManagerComponent_C|GetHotbarWidget _inventorymanager))
  (bind _selectedslotid (Variables|/Game/InventorySystem/UMG/WBP_HotbarWidget.WBP_HotbarWidget_C|GetSelectedSlotID _hotbarwidget))
  (bind _hotbarslots (Variables|/Game/InventorySystem/UMG/WBP_HotbarWidget.WBP_HotbarWidget_C|GetHotbarSlots _hotbarwidget))
  (bind _output (Utilities|Array|Get(acopy) _hotbarslots _selectedslotid))
  ;[1 1 1] The hotbar controls to operate everything to do with the hotbar!!!
  ;;[1 1 1] DoItemDropping
  ;;;[1 1 1] Drop a single item
  (:Pressed
    (Utilities|IsValid _output
      (:Is%20Valid
        (Default|DropItematIndex _inventorymanager (Variables|/Game/InventorySystem/UMG/WBP_HotbarSlot.WBP_HotbarSlot_C|GetSlotID _output) 1)))))

(event Input|KeyboardEvents|1
  (params (Key :type Key%20Structure :default "None"))
  ;[1 1 1] The hotbar controls to operate everything to do with the hotbar!!!
  ;;[1 1 1] Handle 1-9 to select hotbar slots!
  (:Pressed
    (Default|SetSelectedSlot (Variables|/Game/InventorySystem/Blueprints/BP_InventoryManagerComponent.BP_InventoryManagerComponent_C|GetHotbarWidget (Variables|Default|GetInventoryManager)))))

(event Input|KeyboardEvents|2
  (params (Key :type Key%20Structure :default "None"))
  ;[1 1 1] The hotbar controls to operate everything to do with the hotbar!!!
  ;;[1 1 1] Handle 1-9 to select hotbar slots!
  (:Pressed
    (Default|SetSelectedSlot (Variables|/Game/InventorySystem/Blueprints/BP_InventoryManagerComponent.BP_InventoryManagerComponent_C|GetHotbarWidget (Variables|Default|GetInventoryManager)) 1)))

(event Input|KeyboardEvents|3
  (params (Key :type Key%20Structure :default "None"))
  ;[1 1 1] The hotbar controls to operate everything to do with the hotbar!!!
  ;;[1 1 1] Handle 1-9 to select hotbar slots!
  (:Pressed
    (Default|SetSelectedSlot (Variables|/Game/InventorySystem/Blueprints/BP_InventoryManagerComponent.BP_InventoryManagerComponent_C|GetHotbarWidget (Variables|Default|GetInventoryManager)) 2)))

(event Input|KeyboardEvents|4
  (params (Key :type Key%20Structure :default "None"))
  ;[1 1 1] The hotbar controls to operate everything to do with the hotbar!!!
  ;;[1 1 1] Handle 1-9 to select hotbar slots!
  (:Pressed
    (Default|SetSelectedSlot (Variables|/Game/InventorySystem/Blueprints/BP_InventoryManagerComponent.BP_InventoryManagerComponent_C|GetHotbarWidget (Variables|Default|GetInventoryManager)) 3)))

(event Input|KeyboardEvents|5
  (params (Key :type Key%20Structure :default "None"))
  ;[1 1 1] The hotbar controls to operate everything to do with the hotbar!!!
  ;;[1 1 1] Handle 1-9 to select hotbar slots!
  (:Pressed
    (Default|SetSelectedSlot (Variables|/Game/InventorySystem/Blueprints/BP_InventoryManagerComponent.BP_InventoryManagerComponent_C|GetHotbarWidget (Variables|Default|GetInventoryManager)) 4)))

(event Input|KeyboardEvents|6
  (params (Key :type Key%20Structure :default "None"))
  ;[1 1 1] The hotbar controls to operate everything to do with the hotbar!!!
  ;;[1 1 1] Handle 1-9 to select hotbar slots!
  (:Pressed
    (Default|SetSelectedSlot (Variables|/Game/InventorySystem/Blueprints/BP_InventoryManagerComponent.BP_InventoryManagerComponent_C|GetHotbarWidget (Variables|Default|GetInventoryManager)) 5)))

(event Input|KeyboardEvents|7
  (params (Key :type Key%20Structure :default "None"))
  ;[1 1 1] The hotbar controls to operate everything to do with the hotbar!!!
  ;;[1 1 1] Handle 1-9 to select hotbar slots!
  (:Pressed
    (Default|SetSelectedSlot (Variables|/Game/InventorySystem/Blueprints/BP_InventoryManagerComponent.BP_InventoryManagerComponent_C|GetHotbarWidget (Variables|Default|GetInventoryManager)) 6)))

(event Input|KeyboardEvents|8
  (params (Key :type Key%20Structure :default "None"))
  ;[1 1 1] The hotbar controls to operate everything to do with the hotbar!!!
  ;;[1 1 1] Handle 1-9 to select hotbar slots!
  (:Pressed
    (Default|SetSelectedSlot (Variables|/Game/InventorySystem/Blueprints/BP_InventoryManagerComponent.BP_InventoryManagerComponent_C|GetHotbarWidget (Variables|Default|GetInventoryManager)) 7)))

(event Input|KeyboardEvents|9
  (params (Key :type Key%20Structure :default "None"))
  ;[1 1 1] The hotbar controls to operate everything to do with the hotbar!!!
  ;;[1 1 1] Handle 1-9 to select hotbar slots!
  (:Pressed
    (Default|SetSelectedSlot (Variables|/Game/InventorySystem/Blueprints/BP_InventoryManagerComponent.BP_InventoryManagerComponent_C|GetHotbarWidget (Variables|Default|GetInventoryManager)) 8)))

(fn ConstructionScript)