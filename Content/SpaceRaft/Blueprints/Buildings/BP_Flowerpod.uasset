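; Flowerpod building that lets the player plant up to three small plants from the hotbar and water them.
; InteractStart picks the Water or Plant prompt from the held item, checking DT_Items for the SmallPlantable subcategory.
; InteractPress either stores the seed, updates plant meshes and decrements inventory, or wets the dirt.
; Growth is unfinished: watering starts one timer for the first slot, and its PlantDone event is empty.
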(event Custom|RefreshPlants
  (for _index (range 1 (Utilities|Array|Length (Variables|Default|GetPlantedSeeds)))
    (switch int _index
      (:1
        (Components|StaticMesh|SetStaticMesh (Variables|Default|GetPlant) "/Game/ArtistFolder/Byron/Plants/Plant2/p4/p4.p4"))
      (:2
        (Components|StaticMesh|SetStaticMesh (Variables|Default|GetPlant1) "/Game/ArtistFolder/Byron/Plants/Plant2/p4/p4.p4"))
      (:3
        (Components|StaticMesh|SetStaticMesh (Variables|Default|GetPlant2) "/Game/ArtistFolder/Byron/Plants/Plant2/p4/p4.p4")))))

(event Custom|StartPlantTimer
  ;[1 1 1] WOP
  (for _index (range 1 (Utilities|Array|Length (Variables|Default|GetPlantedSeeds)))
    (switch int _index
      (:1
        (Rendering|Material|SetMaterial (Variables|Default|GetDirt) 0 "/Game/ArtistFolder/Gina/Assets/Flowerbed/Materials/MI_DirtWet.MI_DirtWet")
        (Utilities|Time|SetTimerbyEvent (delegate Custom|PlantDone) 3e+01))
      (:2
        (Rendering|Material|SetMaterial (Variables|Default|GetDirt1) 0 "/Game/ArtistFolder/Gina/Assets/Flowerbed/Materials/MI_DirtWet.MI_DirtWet"))
      (:3
        (Rendering|Material|SetMaterial (Variables|Default|GetDirt2) 0 "/Game/ArtistFolder/Gina/Assets/Flowerbed/Materials/MI_DirtWet.MI_DirtWet")))))

(event Custom|PlantDone
  ;[1 1 1] WOP
)

(event EventInteractPress
  (params (Player :type BP%20First%20Person%20Character%20Object%20Reference))
  (bind _itemtoplant (Variables|Default|GetItemToPlant))
  (bind _inventorymanager (Variables|/Game/SpaceRaft/Blueprints/BP_FirstPersonCharacter.BP_FirstPersonCharacter_C|GetInventoryManager Player))
  (bind _hotbarwidget (Variables|/Game/InventorySystem/Blueprints/BP_InventoryManagerComponent.BP_InventoryManagerComponent_C|GetHotbarWidget _inventorymanager))
  (bind _inventory (Variables|/Game/InventorySystem/Blueprints/BP_InventoryManager_Base.BP_InventoryManager_Base_C|GetInventory _inventorymanager))
  (bind _selectedslotid (Variables|/Game/InventorySystem/UMG/WBP_HotbarWidget.WBP_HotbarWidget_C|GetSelectedSlotID _hotbarwidget))
  (bind _output (Utilities|Array|Get(acopy) _inventory _selectedslotid))
  (if (Variables|Default|GetWaterInHand)
    (if (> (Utilities|Array|Length (Variables|Default|GetPlantedSeeds)) 0)
      (CallFunction|StartPlantTimer))
    (elif (not (Utilities|Enum|Equal(Enum) "NewEnumerator2" (Variables|Default|GetItemToPlant)))
      (if (<= (Utilities|Array|Length (Variables|Default|GetPlantedSeeds)) 2)
        (Utilities|Array|Add (Variables|Default|GetPlantedSeeds) _itemtoplant)
        (Utilities|FlowControl|Sequence
          (:then_0
            (CallFunction|RefreshPlants))
          (:then_1
            (bind _result (Math|Integer|DecrementInt (.ammount _output))
              (:%20%20
                (if (<= _result 0)
                  (Utilities|Array|SetArrayElem _inventory _selectedslotid (Utilities|Struct|MakeFInventoryStruct "NewEnumerator2" 0))
                  (Default|ShowItemsChangedWidget _inventorymanager _itemtoplant -1)
                  (Default|SlotUpdate Player _selectedslotid)
                  (else
                    (Utilities|Array|SetArrayElem _inventory _selectedslotid (Utilities|Struct|MakeFInventoryStruct (.item _output) _result))))))))
        (else
          (bind _validinteraction_ (CallFunction|InteractStart (Variables|Default|GetItemToPlant)))
          (if (not _validinteraction_)
            (bind _asbp_spaft_hud (Utilities|Casting|CastToBP_SpaftHud (HUD|GetHUD (Game|GetPlayerController 0))))
            (Default|HideInteraction (Variables|/Game/SpaceRaft/Game/BP_SpaftHud.BP_SpaftHud_C|GetWBPInteractNotify _asbp_spaft_hud))))))))

(fn ConstructionScript)

(fn InteractStart
  (params (HeldItem :type EItems%20Enum :default "NewEnumerator0"))
  (if (Utilities|Enum|Equal(Enum) HeldItem "NewEnumerator13")
    (if (> (Utilities|Array|Length (Variables|Default|GetPlantedSeeds)) 0)
      (Variables|Default|SetWaterInHand true)
      (return "Water" true)
      (else
        (return "" false)))
    (else
      (Variables|Default|SetWaterInHand false)
      (bind _outrownames (DataTable|GetDataTableRowNames "/Game/InventorySystem/Datatables/DT_Items.DT_Items"))
      (for _array_element _outrownames
        (bind _returnvalue (Utilities|GetDataTableRow "/Game/InventorySystem/Datatables/DT_Items.DT_Items" _array_element)
          (:then
            (if (and (Utilities|Enum|Equal(Enum) HeldItem (.item _returnvalue)) (== (.subcategory _returnvalue) "SmallPlantable"))
              (Variables|Default|SetItemToPlant HeldItem)
              (if (<= (Utilities|Array|Length (Variables|Default|GetPlantedSeeds)) 3)
                (return "Plant" true)
                (else
                  _)))
            (return "" false)))))))