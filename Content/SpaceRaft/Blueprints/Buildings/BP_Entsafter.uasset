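; BP_Entsafter is a juicer building that squishes a usable held item and then fills a specific held item with the result.
; InteractStart picks the prompt from production state and held item and caches ItemToAdd, which InteractPress relies on.
; InteractPress edits the player's selected hotbar slot and starts production on a fixed timer.
; Material swaps show idle, working and finished states, and finishing refreshes the HUD prompt.
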(event Custom|Production
  (Utilities|Time|SetTimerbyEvent (delegate Custom|FinishProduction) 5.0))

(event Custom|FinishProduction
  (bind _returnvalue (Game|GetPlayerController 0))
  (bind _returnvalue_2 (HUD|GetHUD _returnvalue))
  (Variables|Default|SetItemInside "NewEnumerator2")
  (Variables|Default|SetProductionState "NewEnumerator2")
  (Rendering|Material|SetMaterial (Variables|Default|GetStaticMesh) 2 "/Game/SpaceRaft/Objects/Entsafter/Entsafter_Finished.Entsafter_Finished")
  (bind _asbp_first_person_character (Utilities|Casting|CastToBP_FirstPersonCharacter (Game|Player|GetPlayerPawn 0)))
  (bind (_text _validinteraction_) (CallFunction|InteractStart (Variables|/Game/SpaceRaft/Blueprints/BP_FirstPersonCharacter.BP_FirstPersonCharacter_C|GetHeldItem _asbp_first_person_character)))
  (if _validinteraction_
    (bind _asbp_spaft_hud (Utilities|Casting|CastToBP_SpaftHud _returnvalue_2))
    (Default|ShowInteraction (Variables|/Game/SpaceRaft/Game/BP_SpaftHud.BP_SpaftHud_C|GetWBPInteractNotify _asbp_spaft_hud) _text)
    (else
      (bind _asbp_spaft_hud_2 (Utilities|Casting|CastToBP_SpaftHud _returnvalue_2))
      (Default|HideInteraction (Variables|/Game/SpaceRaft/Game/BP_SpaftHud.BP_SpaftHud_C|GetWBPInteractNotify _asbp_spaft_hud_2)))))

(event EventInteractPress
  (params (Player :type BP%20First%20Person%20Character%20Object%20Reference))
  (bind _inventorymanager (Variables|/Game/SpaceRaft/Blueprints/BP_FirstPersonCharacter.BP_FirstPersonCharacter_C|GetInventoryManager Player))
  (bind _inventorymanager_2 (Variables|/Game/SpaceRaft/Blueprints/BP_FirstPersonCharacter.BP_FirstPersonCharacter_C|GetInventoryManager Player))
  (bind _inventory (Variables|/Game/InventorySystem/Blueprints/BP_InventoryManager_Base.BP_InventoryManager_Base_C|GetInventory _inventorymanager_2))
  (bind _hotbarwidget (Variables|/Game/InventorySystem/Blueprints/BP_InventoryManagerComponent.BP_InventoryManagerComponent_C|GetHotbarWidget _inventorymanager_2))
  (bind _hotbarwidget_2 (Variables|/Game/InventorySystem/Blueprints/BP_InventoryManagerComponent.BP_InventoryManagerComponent_C|GetHotbarWidget _inventorymanager))
  (bind _selectedslotid (Variables|/Game/InventorySystem/UMG/WBP_HotbarWidget.WBP_HotbarWidget_C|GetSelectedSlotID _hotbarwidget))
  (bind _selectedslotid_2 (Variables|/Game/InventorySystem/UMG/WBP_HotbarWidget.WBP_HotbarWidget_C|GetSelectedSlotID _hotbarwidget_2))
  (bind _output (Utilities|Array|Get(acopy) _inventory _selectedslotid))
  (if (and (Utilities|Enum|Equal(Enum) (Variables|Default|GetProductionState) "NewEnumerator2") (Utilities|Enum|Equal(Enum) (Variables|/Game/SpaceRaft/Blueprints/BP_FirstPersonCharacter.BP_FirstPersonCharacter_C|GetHeldItem Player) "NewEnumerator12"))
    (Utilities|Array|SetArrayElem (Variables|/Game/InventorySystem/Blueprints/BP_InventoryManager_Base.BP_InventoryManager_Base_C|GetInventory _inventorymanager) _selectedslotid_2 (Utilities|Struct|MakeFInventoryStruct "NewEnumerator13" 1))
    (Default|SlotUpdate Player _selectedslotid_2)
    (Variables|Default|SetProductionState "NewEnumerator0")
    (Rendering|Material|SetMaterial (Variables|Default|GetStaticMesh) 2 "/Game/SpaceRaft/Objects/Entsafter/Entsafter_Idle.Entsafter_Idle")
    (elif (not (Utilities|Enum|Equal(Enum) (Variables|Default|GetProductionState) "NewEnumerator1"))
      (if (not (Utilities|Enum|Equal(Enum) (Variables|Default|GetItemToAdd) "NewEnumerator2"))
        (Variables|Default|SetItemInside (Variables|Default|GetItemToAdd))
        (Variables|Default|SetProductionState "NewEnumerator1")
        (CallFunction|Production)
        (Rendering|Material|SetMaterial (Variables|Default|GetStaticMesh) 2 "/Game/SpaceRaft/Objects/Entsafter/Entsafter_Working.Entsafter_Working")
        (bind _result (Math|Integer|DecrementInt (.ammount _output))
          (:%20%20
            (if (<= _result 0)
              (Utilities|Array|SetArrayElem _inventory _selectedslotid (Utilities|Struct|MakeFInventoryStruct "NewEnumerator2" 0))
              (Default|ShowItemsChangedWidget _inventorymanager_2 (Variables|Default|GetItemToAdd) -1)
              (Default|SlotUpdate Player _selectedslotid)
              (else
                (Utilities|Array|SetArrayElem _inventory _selectedslotid (Utilities|Struct|MakeFInventoryStruct (.item _output) _result))))))))))

(fn ConstructionScript)

(fn InteractStart
  (params (HeldItem :type EItems%20Enum :default "NewEnumerator0"))
  (if (not (Utilities|Enum|Equal(Enum) (Variables|Default|GetProductionState) "NewEnumerator0"))
    (if (Utilities|Enum|Equal(Enum) (Variables|Default|GetProductionState) "NewEnumerator2")
      (if (Utilities|Enum|Equal(Enum) HeldItem "NewEnumerator12")
        (return "Fill" true)
        (else
          _)))
    (elif (Utilities|Array|ContainsItem (LocalVariables|GetUsableItems) HeldItem)
      (if (Utilities|Enum|NotEqual(Enum) (Variables|Default|GetItemInside) "NewEnumerator2")
        _
        (else
          (Variables|Default|SetItemToAdd HeldItem)
          (return "Squish" true)))))
  (Variables|Default|SetItemToAdd "NewEnumerator2")
  (return "" false))