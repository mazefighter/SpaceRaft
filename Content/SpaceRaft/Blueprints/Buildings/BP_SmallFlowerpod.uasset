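; BP_SmallFlowerpod is an interactable planter building where the player plants an item, waters it and harvests it.
; InteractStart picks the Plant, Water or Take prompt from production state and held item, and InteractPress updates the hotbar inventory, meshes and soil material.
; Watering starts a looping timer that randomly scales up the plant until a five-second timer finishes production.
; Taking yields a random amount of the planted item and resets the pod.
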(event Custom|Production
  (bind _returnvalue (Utilities|Time|SetTimerbyEvent (delegate Custom|SeedGrow) 0.1 true))
  (Utilities|Time|SetTimerbyEvent (delegate Custom|FinishProduction) 5.0))

(event Custom|FinishProduction
  (bind _returnvalue (Game|GetPlayerController 0))
  (bind _returnvalue_2 (HUD|GetHUD _returnvalue))
  (Utilities|Time|ClearandInvalidateTimerbyHandle (stale Custom|Production _returnvalue))
  (Variables|Default|SetProductionState "NewEnumerator2")
  (bind _asbp_first_person_character (Utilities|Casting|CastToBP_FirstPersonCharacter (Game|Player|GetPlayerPawn 0)))
  (bind (_text _validinteraction_) (CallFunction|InteractStart (Variables|/Game/SpaceRaft/Blueprints/BP_FirstPersonCharacter.BP_FirstPersonCharacter_C|GetHeldItem _asbp_first_person_character)))
  (if _validinteraction_
    (bind _asbp_spaft_hud (Utilities|Casting|CastToBP_SpaftHud _returnvalue_2))
    (Default|ShowInteraction (Variables|/Game/SpaceRaft/Game/BP_SpaftHud.BP_SpaftHud_C|GetWBPInteractNotify _asbp_spaft_hud) _text)
    (else
      (bind _asbp_spaft_hud_2 (Utilities|Casting|CastToBP_SpaftHud _returnvalue_2))
      (Default|HideInteraction (Variables|/Game/SpaceRaft/Game/BP_SpaftHud.BP_SpaftHud_C|GetWBPInteractNotify _asbp_spaft_hud_2)))))

(event Custom|SeedGrow
  (bind _output_get (Variables|Default|SetPlantScale (+ (Variables|Default|GetPlantScale) (* (Utilities|Time|GetWorldDeltaSeconds) (Math|Random|RandomFloatinRange 1.0 4.0)))))
  (Transformation|SetRelativeScale3D (Variables|Default|GetStaticMesh1) (Math|Vector|MakeVector _output_get _output_get _output_get)))

(event EventBeginPlay)

(event Collision|EventActorBeginOverlap
  (params (OtherActor :type Actor%20Object%20Reference)))

(event EventTick
  (params (DeltaSeconds :type Float%20%28single-precision%29)))

(event EventInteractPress
  (params (Player :type BP%20First%20Person%20Character%20Object%20Reference))
  (bind _returnvalue (Game|GetPlayerController 0))
  (bind _inventorymanager (Variables|/Game/SpaceRaft/Blueprints/BP_FirstPersonCharacter.BP_FirstPersonCharacter_C|GetInventoryManager Player))
  (bind _inventorymanager_2 (Variables|/Game/SpaceRaft/Blueprints/BP_FirstPersonCharacter.BP_FirstPersonCharacter_C|GetInventoryManager Player))
  (bind _inventorymanager_3 (Variables|/Game/SpaceRaft/Blueprints/BP_FirstPersonCharacter.BP_FirstPersonCharacter_C|GetInventoryManager Player))
  (bind _returnvalue_2 (HUD|GetHUD _returnvalue))
  (bind _inventory (Variables|/Game/InventorySystem/Blueprints/BP_InventoryManager_Base.BP_InventoryManager_Base_C|GetInventory _inventorymanager_3))
  (bind _hotbarwidget (Variables|/Game/InventorySystem/Blueprints/BP_InventoryManagerComponent.BP_InventoryManagerComponent_C|GetHotbarWidget _inventorymanager_3))
  (bind _selectedslotid (Variables|/Game/InventorySystem/UMG/WBP_HotbarWidget.WBP_HotbarWidget_C|GetSelectedSlotID _hotbarwidget))
  (bind _output (Utilities|Array|Get(acopy) _inventory _selectedslotid))
  (if (Utilities|Enum|Equal(Enum) (Variables|Default|GetProductionState) "NewEnumerator2")
    (Default|AddItem _inventorymanager_2 (Variables|Default|GetItemPlanted) (Math|Random|RandomIntegerinRange 2 4))
    (Default|SlotUpdate Player (Variables|/Game/InventorySystem/UMG/WBP_HotbarWidget.WBP_HotbarWidget_C|GetSelectedSlotID (Variables|/Game/InventorySystem/Blueprints/BP_InventoryManagerComponent.BP_InventoryManagerComponent_C|GetHotbarWidget _inventorymanager_2)))
    (Variables|Default|SetProductionState "NewEnumerator0")
    (Variables|Default|SetPlanted false)
    (Variables|Default|SetItemPlanted "NewEnumerator2")
    (bind _output_get (Variables|Default|SetPlantScale 0.1))
    (Transformation|SetRelativeScale3D (Variables|Default|GetStaticMesh1) (Math|Vector|MakeVector _output_get _output_get _output_get))
    (Components|StaticMesh|SetStaticMesh (Variables|Default|GetStaticMesh1) 0)
    (Rendering|Material|SetMaterial (Variables|Default|GetStaticMesh) 1 "/Game/ArtistFolder/Gina/Assets/Flowerbed/Materials/MI_Dirt.MI_Dirt")
    (elif (not (Utilities|Enum|Equal(Enum) (Variables|Default|GetProductionState) "NewEnumerator1"))
      (if (not (Utilities|Enum|Equal(Enum) (Variables|Default|GetItemToAdd) "NewEnumerator2"))
        (if (not (Variables|Default|GetPlanted))
          (Variables|Default|SetItemPlanted (Variables|Default|GetItemToAdd))
          (Variables|Default|SetPlanted true)
          (Components|StaticMesh|SetStaticMesh (Variables|Default|GetStaticMesh1) "/Game/ArtistFolder/Byron/Plants/Plant2/p4/p4.p4")
          (bind _result (Math|Integer|DecrementInt (.ammount _output))
            (:%20%20
              (if (<= _result 0)
                (Utilities|Array|SetArrayElem _inventory _selectedslotid (Utilities|Struct|MakeFInventoryStruct "NewEnumerator2" 0))
                (else
                  (Utilities|Array|SetArrayElem _inventory _selectedslotid (Utilities|Struct|MakeFInventoryStruct (.item _output) _result))))
              (Default|ShowItemsChangedWidget _inventorymanager_3 (Variables|Default|GetItemToAdd) -1)
              (Default|SlotUpdate Player _selectedslotid)
              (bind _asbp_first_person_character (Utilities|Casting|CastToBP_FirstPersonCharacter (Game|Player|GetPlayerPawn 0) :!label _label))
              (bind (_text _validinteraction_) (CallFunction|InteractStart (Variables|/Game/SpaceRaft/Blueprints/BP_FirstPersonCharacter.BP_FirstPersonCharacter_C|GetHeldItem _asbp_first_person_character)))
              (if _validinteraction_
                (bind _asbp_spaft_hud (Utilities|Casting|CastToBP_SpaftHud _returnvalue_2))
                (Default|ShowInteraction (Variables|/Game/SpaceRaft/Game/BP_SpaftHud.BP_SpaftHud_C|GetWBPInteractNotify _asbp_spaft_hud) _text)
                (else
                  (bind _asbp_spaft_hud_2 (Utilities|Casting|CastToBP_SpaftHud _returnvalue_2))
                  (Default|HideInteraction (Variables|/Game/SpaceRaft/Game/BP_SpaftHud.BP_SpaftHud_C|GetWBPInteractNotify _asbp_spaft_hud_2))))))
          (elif (Utilities|Enum|Equal(Enum) (Variables|/Game/SpaceRaft/Blueprints/BP_FirstPersonCharacter.BP_FirstPersonCharacter_C|GetHeldItem Player) "NewEnumerator13")
            (Variables|Default|SetProductionState "NewEnumerator1")
            (CallFunction|Production)
            (Utilities|Array|SetArrayElem (Variables|/Game/InventorySystem/Blueprints/BP_InventoryManager_Base.BP_InventoryManager_Base_C|GetInventory _inventorymanager) (Variables|/Game/InventorySystem/UMG/WBP_HotbarWidget.WBP_HotbarWidget_C|GetSelectedSlotID (Variables|/Game/InventorySystem/Blueprints/BP_InventoryManagerComponent.BP_InventoryManagerComponent_C|GetHotbarWidget _inventorymanager)) (Utilities|Struct|MakeFInventoryStruct "NewEnumerator12" 1))
            (Rendering|Material|SetMaterial (Variables|Default|GetStaticMesh) 1 "/Game/ArtistFolder/Gina/Assets/Flowerbed/Materials/MI_DirtWet.MI_DirtWet")
            (goto _label)))))))

(fn ConstructionScript)

(fn InteractStart
  (params (HeldItem :type EItems%20Enum :default "NewEnumerator0"))
  (if (not (Utilities|Enum|Equal(Enum) (Variables|Default|GetProductionState) "NewEnumerator0"))
    (if (Utilities|Enum|Equal(Enum) (Variables|Default|GetProductionState) "NewEnumerator2")
      (return "Take" true)
      (else
        _))
    (elif (Variables|Default|GetPlanted)
      (if (Utilities|Enum|Equal(Enum) HeldItem "NewEnumerator13")
        (Variables|Default|SetItemToAdd HeldItem)
        (return "Water" true)
        (else
          _))
      (elif (Utilities|Array|ContainsItem (LocalVariables|GetUsableItems) HeldItem)
        (if (Utilities|Enum|NotEqual(Enum) (Variables|Default|GetItemPlanted) "NewEnumerator2")
          _
          (else
            (Variables|Default|SetItemToAdd HeldItem)
            (return "Plant" true))))))
  (Variables|Default|SetItemToAdd "NewEnumerator2")
  (return "" false))