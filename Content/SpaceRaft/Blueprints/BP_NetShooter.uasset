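; BP_NetShooter is a possessable net launcher with look controls that fires a net at debris, using its own Enhanced Input mapping.
; Holding ShootNet runs a charge timeline, and releasing it saves the strength that scales a second timeline extending the spring arm.
; Overlapping BP_Debris stops the extension.
; Both that stop and a completed forward shot lead into a short delay with nothing after it, so no retraction happens here.
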(event OnComponentBeginOverlap(Net)
  (params (OverlappedComponent :type Primitive%20Component%20Object%20Reference) (OtherActor :type Actor%20Object%20Reference) (OtherComp :type Primitive%20Component%20Object%20Reference) (OtherBodyIndex :type Integer) (bFromSweep :type Boolean) (SweepResult :type Hit%20Result%20Structure%20%28by%20ref%29))
  (Utilities|Casting|CastToBP_Debris OtherActor)
  (Utilities|FlowControl|Sequence
    (:then_0
      (bind (_direction _armlenght) (Timeline|ShootArm Stop)
        (:Update
          (Variables|/Script/Engine.SpringArmComponent|SetTargetArmLength (Variables|Default|GetSpringArm) (* _armlenght (Variables|Default|GetNetStrength))))
        (:Finished
          (switch Utilities|FlowControl|Switch|SwitchonETimelineDirection _direction
            (:Forward
              (CallFunction|ReverseTimer))))))
    (:then_1
      (Utilities|FlowControl|Delay 0.4))))

(event Custom|Reverse%20Timer
  (Utilities|FlowControl|Delay 0.4))

(event Input|EnhancedActionEvents|EnhancedInputActionShootNet
  (params (ActionValue :type Boolean) (ElapsedSeconds :type Float%20%28double-precision%29) (TriggeredSeconds :type Float%20%28double-precision%29) (InputAction :type Input%20Action%20Object%20Reference :default "/Game/SpaceRaft/Inputs/Actions/ShootNet.ShootNet"))
  (:Started
    (Variables|Default|SetNetStrength 0.0)
    (bind _netshoot (Timeline|Strenght PlayFromStart)))
  (:Completed
    (Utilities|FlowControl|Sequence
      (:then_0
        (Timeline|Strenght Stop))
      (:then_1
        (Variables|Default|SetNetStrength _netshoot))
      (:then_2
        (bind (_direction _armlenght) (Timeline|ShootArm PlayFromStart)
          (:Update
            (Variables|/Script/Engine.SpringArmComponent|SetTargetArmLength (Variables|Default|GetSpringArm) (* _armlenght (Variables|Default|GetNetStrength))))
          (:Finished
            (switch Utilities|FlowControl|Switch|SwitchonETimelineDirection _direction
              (:Forward
                (CallFunction|ReverseTimer)))))))))

(event Input|EnhancedActionEvents|EnhancedInputActionIA_Look
  (params (ActionValue :type Vector%202D%20Structure) (ElapsedSeconds :type Float%20%28double-precision%29) (TriggeredSeconds :type Float%20%28double-precision%29) (InputAction :type Input%20Action%20Object%20Reference :default "/Game/SpaceRaft/Inputs/Actions/IA_Look.IA_Look"))
  (Pawn|Input|AddControllerYawInput (.x ActionValue))
  (Pawn|Input|AddControllerPitchInput (.y ActionValue)))

(event EventBeginPlay)

(event EventPossessed
  (params (NewController :type Controller%20Object%20Reference))
  (bind _asplayer_controller (Utilities|Casting|CastToPlayerController (Pawn|GetController)))
  (Utilities|IsValid (PlayerController|LocalPlayerSubsystems|GetEnhancedInputLocalPlayerSubsystem _asplayer_controller)
    (:Is%20Valid
      (Class|EnhancedInputSubsystemInterface|ClearAllMappings (PlayerController|LocalPlayerSubsystems|GetEnhancedInputLocalPlayerSubsystem _asplayer_controller))
      (Input|AddMappingContext (PlayerController|LocalPlayerSubsystems|GetEnhancedInputLocalPlayerSubsystem _asplayer_controller) "/Game/SpaceRaft/Inputs/NetShooter.NetShooter" 0 "(bIgnoreAllPressedKeysUntilRelease=True,bForceImmediately=False,bNotifyUserSettings=False)"))))

(event EventTick
  (params (DeltaSeconds :type Float%20%28single-precision%29)))

(event Collision|EventActorBeginOverlap
  (params (OtherActor :type Actor%20Object%20Reference)))

(fn ConstructionScript)