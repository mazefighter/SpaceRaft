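; BP_Debris is a drifting space debris actor for SpaceRaft that carries a randomly chosen item type.
; BeginPlay randomizes mesh rotation, picks a mesh and Item through weighted integer ranges, rolls a speed and starts a timed self-destruct.
; Tick moves it opposite its forward vector, using DeltaSeconds as a transform lerp alpha for frame-scaled motion.
; Overlapping a BP_Spacecraft with the mesh destroys it.
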(event OnComponentBeginOverlap(Mesh)
  (params (OverlappedComponent :type Primitive%20Component%20Object%20Reference) (OtherActor :type Actor%20Object%20Reference) (OtherComp :type Primitive%20Component%20Object%20Reference) (OtherBodyIndex :type Integer) (bFromSweep :type Boolean) (SweepResult :type Hit%20Result%20Structure%20%28by%20ref%29))
  (Utilities|Casting|CastToBP_Spacecraft OtherActor)
  (Actor|DestroyActor))

(event Custom|Destory%20Actor
  (Actor|DestroyActor))

(event EventBeginPlay
  (bind _mesh (Variables|Default|GetMesh))
  (Transformation|SetRelativeRotation (Variables|Default|GetMesh) (Math|Random|RandomRotator true) false false)
  (Variables|Default|SetRandomInt (Math|Random|RandomIntegerinRange 0 100))
  (if (Math|Integer|InRange(Integer) (Variables|Default|GetRandomInt) 0 5 true false)
    (Components|StaticMesh|SetStaticMesh _mesh "/Game/ArtistFolder/Gina/Assets/Scrap/Capsule/Kapsel_01.Kapsel_01")
    (Variables|Default|SetItem "NewEnumerator0")
    (elif (Math|Integer|InRange(Integer) (Variables|Default|GetRandomInt) 5 25 true false)
      (Components|StaticMesh|SetStaticMesh _mesh "/Game/ArtistFolder/Gina/Assets/Scrap/cable/cable_02.cable_02")
      (Variables|Default|SetItem "NewEnumerator11")
      (elif (Math|Integer|InRange(Integer) (Variables|Default|GetRandomInt) 25 50 true false)
        (Components|StaticMesh|SetStaticMesh _mesh "/Game/ArtistFolder/Gina/Assets/Scrap/Bottle/v2/opt_bottle.opt_bottle")
        (Variables|Default|SetItem "NewEnumerator10")
        (elif (Math|Integer|InRange(Integer) (Variables|Default|GetRandomInt) 50 70 true false)
          (Components|StaticMesh|SetStaticMesh _mesh "/Game/ArtistFolder/Gina/Assets/Scrap/Pipe/Metal_Pipe_04.Metal_Pipe_04")
          (Variables|Default|SetItem "NewEnumerator8")
          (elif (Math|Integer|InRange(Integer) (Variables|Default|GetRandomInt) 70 100)
            (Components|StaticMesh|SetStaticMesh _mesh "/Game/ArtistFolder/Gina/Assets/Scrap/Plates/Metal_Plates_02.Metal_Plates_02")
            (Variables|Default|SetItem "NewEnumerator8"))))))
  (Utilities|Time|SetTimerbyEvent (delegate Custom|Destory%20Actor) 9e+01)
  (Variables|Default|SetSpeed (Math|Random|RandomFloatinRange (Variables|Default|GetSpeedMin) (Variables|Default|GetSpeedmax))))

(event Collision|EventActorBeginOverlap
  (params (OtherActor :type Actor%20Object%20Reference)))

(event EventTick
  (params (DeltaSeconds :type Float%20%28single-precision%29))
  (bind _returnvalue (Transformation|GetActorTransform))
  (bind (_location _rotation _scale) (Math|Transform|BreakTransform _returnvalue))
  (Transformation|SetActorTransform (Math|Transform|Lerp(Transform) _returnvalue (Math|Transform|MakeTransform (+ _location (Math|Vector|NegateVector (* (Transformation|GetActorForwardVector) (Variables|Default|GetSpeed)))) _rotation _scale) DeltaSeconds)))

(fn ConstructionScript)