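; BP_PosessNetShooter is an interactable that puts the player in control of the level's net shooter.
; On BeginPlay it caches the BP_NetShooter found with GetActorOfClass.
; InteractStart always reports a valid interaction with a "Use" prompt, and InteractPress makes player controller 0 possess the cached net shooter.
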(event EventBeginPlay
  (bind _returnvalue (Actor|GetActorOfClass "/Game/SpaceRaft/Blueprints/BP_NetShooter.BP_NetShooter_C"))
  (Variables|Default|SetBP_NetShooter _returnvalue))

(event Collision|EventActorBeginOverlap
  (params (OtherActor :type Actor%20Object%20Reference)))

(event EventTick
  (params (DeltaSeconds :type Float%20%28single-precision%29)))

(event EventInteractPress
  (params (Player :type BP%20First%20Person%20Character%20Object%20Reference))
  (Pawn|Possess (Game|GetPlayerController 0) (Variables|Default|GetBP_NetShooter)))

(fn ConstructionScript)

(fn InteractStart
  (params (HeldItem :type EItems%20Enum :default "NewEnumerator0"))
  (return "Use" true))