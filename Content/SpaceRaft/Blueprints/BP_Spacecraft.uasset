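; BP_Spacecraft is the spacecraft Blueprint, which continuously spawns BP_Debris actors during play.
; BeginPlay starts a looping timer at SpawnRate that fires the SpawnDebris event.
; Each debris actor appears at a random point on a fixed-radius sphere around the DebrisSpawner component, oriented to the craft's rotation with slight random jitter on each axis.
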(event Custom|Spawn%20Debris
  (bind _returnvalue (Transformation|GetActorRotation))
  (Game|SpawnActorfromClass "/Game/SpaceRaft/Blueprints/BP_Debris.BP_Debris_C" (Math|Transform|MakeTransform (+ (Transformation|GetWorldLocation (Variables|Default|GetDebrisSpawner)) (* (Math|Random|RandomUnitVector) 4e+03)) (Math|Rotator|MakeRotator (+ (.roll _returnvalue) (Math|Random|RandomFloatinRange -3.0 3.0)) (+ (.pitch _returnvalue) (Math|Random|RandomFloatinRange -3.0 3.0)) (+ (.yaw _returnvalue) (Math|Random|RandomFloatinRange -3.0 3.0))) "1.000000,1.000000,1.000000") "Undefined" "MultiplyWithRoot" 0 0))

(event EventBeginPlay
  (Utilities|Time|SetTimerbyEvent (delegate Custom|Spawn%20Debris) (Variables|Default|GetSpawnRate) true))

(event EventTick
  (params (DeltaSeconds :type Float%20%28single-precision%29)))

(fn ConstructionScript)