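; BP_Flowerpod is an interactable planter in SpaceRaft that stores up to four planted items.
; InteractStart accepts only Apple or Pear, caches it as ItemToPlant and returns the "Plant" prompt while space remains.
; InteractPress adds the cached item to PlantedSeeds and decrements the player's selected hotbar stack, clearing emptied slots.
; Pressing when full rechecks validity and hides the HUD interaction prompt; no growth logic exists here.
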(event EventBeginPlay)

(event Collision|EventActorBeginOverlap
  (params (OtherActor :type Actor%20Object%20Reference)))

(event EventTick
  (params (DeltaSeconds :type Float%20%28single-precision%29)))

(event EventInteractPress
  (params (Player :type BP%20First%20Person%20Character%20Object%20Reference))
  (bind _inventorymanager (Variables|/Game/SpaceRaft/Blueprints/BP_FirstPersonCharacter.BP_FirstPersonCharacter_C|GetInventoryManager Player))
  (bind _hotbarwidget (Variables|/Game/InventorySystem/Blueprints/BP_InventoryManagerComponent.BP_InventoryManagerComponent_C|GetHotbarWidget _inventorymanager))
  (bind _inventory (Variables|/Game/InventorySystem/Blueprints/BP_InventoryManager_Base.BP_InventoryManager_Base_C|GetInventory _inventorymanager))
  (bind _selectedslotid (Variables|/Game/InventorySystem/UMG/WBP_HotbarWidget.WBP_HotbarWidget_C|GetSelectedSlotID _hotbarwidget))
  (bind _output (Utilities|Array|Get(acopy) _inventory _selectedslotid))
  (if (not (Utilities|Enum|Equal(Enum) "NewEnumerator2" (Variables|Default|GetItemToPlant)))
    (if (<= (Utilities|Array|Length (Variables|Default|GetPlantedSeeds)) 3)
      (Utilities|Array|Add (Variables|Default|GetPlantedSeeds) (Variables|Default|GetItemToPlant))
      (bind _result (Math|Integer|DecrementInt (.ammount _output))
        (:%20%20
          (if (<= _result 0)
            (Utilities|Array|SetArrayElem _inventory _selectedslotid (Utilities|Struct|MakeFInventoryStruct "NewEnumerator2" 0))
            (Default|SlotUpdate Player _selectedslotid)
            (else
              (Utilities|Array|SetArrayElem _inventory _selectedslotid (Utilities|Struct|MakeFInventoryStruct (.item _output) _result))))))
      (else
        (bind _validinteraction_ (CallFunction|InteractStart (Variables|Default|GetItemToPlant)))
        (if (not _validinteraction_)
          (bind _asbp_spaft_hud (Utilities|Casting|CastToBP_SpaftHud (HUD|GetHUD (Game|GetPlayerController 0))))
          (Default|HideInteraction (Variables|/Game/SpaceRaft/Game/BP_SpaftHud.BP_SpaftHud_C|GetWBPInteractNotify _asbp_spaft_hud)))))))

(fn ConstructionScript)

(fn InteractStart
  (params (HeldItem :type EItems%20Enum :default "NewEnumerator0"))
  (switch Utilities|FlowControl|Switch|SwitchonEItems HeldItem
    (:NewEnumerator0
      (Variables|Default|SetItemToPlant HeldItem :!label _label)
      (if (<= (Utilities|Array|Length (Variables|Default|GetPlantedSeeds)) 3)
        _
        (else
          (return "" false))))
    (:NewEnumerator1
      (return "" false))
    (:NewEnumerator3
      (goto _label))
    (:NewEnumerator5
      (return "" false))
    (:NewEnumerator4
      (return "" false))
    (:NewEnumerator6
      (return "" false))
    (:NewEnumerator7
      (return "" false))
    (:NewEnumerator2
      (return "" false)))
  (return "Plant" true))