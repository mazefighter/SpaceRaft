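; BP_SpaftHud is the HUD for the SpaceRaft game, creating the on-screen UI when play begins.
; BeginPlay creates the net turret, interact notify, survival and exit game widgets, adds each to the viewport and stores a reference.
; The interact notify and exit game widgets start hidden, and this Blueprint contains no logic to show them or update any widget.
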(event EventBeginPlay
  (Utilities|FlowControl|Sequence
    (:then_0
      (bind _returnvalue (UserInterface|CreateWidget "/Game/SpaceRaft/UI/TurretUI/WBP_NetTurretUI.WBP_NetTurretUI_C"))
      (UserInterface|Viewport|AddtoViewport _returnvalue 0)
      (Variables|Default|SetWBPNetTurretUI _returnvalue))
    (:then_1
      (bind _returnvalue_2 (UserInterface|CreateWidget "/Game/SpaceRaft/UI/InventoryUI/WBP_InteractNotify.WBP_InteractNotify_C"))
      (UserInterface|Viewport|AddtoViewport _returnvalue_2 0)
      (bind _output_get (Variables|Default|SetWBPInteractNotify _returnvalue_2))
      (Widget|SetVisibility _output_get "Hidden"))
    (:then_2
      (bind _returnvalue_3 (UserInterface|CreateWidget "/Game/SpaceRaft/UI/SurvivalUI/WBP_Survival.WBP_Survival_C"))
      (UserInterface|Viewport|AddtoViewport _returnvalue_3 0)
      (Variables|Default|SetWBPSurvival _returnvalue_3))
    (:then_3
      (bind _returnvalue_4 (UserInterface|CreateWidget "/Game/SpaceRaft/UI/WBP_ExitGame.WBP_ExitGame_C"))
      (UserInterface|Viewport|AddtoViewport _returnvalue_4 0)
      (bind _output_get_2 (Variables|Default|SetWBPExit _returnvalue_4))
      (Widget|SetVisibility _output_get_2 "Hidden"))))

(event Collision|EventActorBeginOverlap
  (params (OtherActor :type Actor%20Object%20Reference)))

(event EventTick
  (params (DeltaSeconds :type Float%20%28single-precision%29)))

(fn ConstructionScript)