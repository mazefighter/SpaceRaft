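; Game instance for SpaceRaft that saves and loads the time leaderboard through a BP_SaveLeaderboard save object.
; SaveAndClose loads or creates the GameSave slot, appends the name and two-digit minute and second texts to parallel arrays, saves, then opens the Menu level.
; Load returns those three arrays when a save exists.
; Entries are stored in insertion order, with no sorting.
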(fn SaveandClose
  (params (Name :type Text) (Minutes :type Integer) (Seconds :type Integer))
  (bind _returnvalue (Utilities|Text|ToText(Integer) Seconds false true 2 2))
  (bind _returnvalue_2 (Utilities|Text|ToText(Integer) Minutes false true 2 2))
  (bind _returnvalue_3 (SaveGame|DoesSaveGameExist "GameSave"))
  (if _returnvalue_3
    (bind _returnvalue_4 (SaveGame|LoadGamefromSlot "Gamesave"))
    (bind _asbp_save_leaderboard (Utilities|Casting|CastToBP_SaveLeaderboard _returnvalue_4))
    (Utilities|Array|Add (Variables|/Game/SpaceRaft/Blueprints/BP_SaveLeaderboard.BP_SaveLeaderboard_C|GetName _asbp_save_leaderboard) Name)
    (Utilities|Array|Add (Variables|/Game/SpaceRaft/Blueprints/BP_SaveLeaderboard.BP_SaveLeaderboard_C|GetMinutes _asbp_save_leaderboard) _returnvalue_2)
    (Utilities|Array|Add (Variables|/Game/SpaceRaft/Blueprints/BP_SaveLeaderboard.BP_SaveLeaderboard_C|GetSeconds _asbp_save_leaderboard) _returnvalue)
    (SaveGame|SaveGametoSlot _asbp_save_leaderboard "GameSave")
    (Game|OpenLevel(byObjectReference) "/Game/ArtistFolder/Byron/Menu.Menu")
    (else
      (bind _returnvalue_5 (SaveGame|CreateSaveGameObject "/Game/SpaceRaft/Blueprints/BP_SaveLeaderboard.BP_SaveLeaderboard_C"))
      (Utilities|Array|Add (Variables|/Game/SpaceRaft/Blueprints/BP_SaveLeaderboard.BP_SaveLeaderboard_C|GetName _returnvalue_5) Name)
      (Utilities|Array|Add (Variables|/Game/SpaceRaft/Blueprints/BP_SaveLeaderboard.BP_SaveLeaderboard_C|GetMinutes _returnvalue_5) _returnvalue_2)
      (Utilities|Array|Add (Variables|/Game/SpaceRaft/Blueprints/BP_SaveLeaderboard.BP_SaveLeaderboard_C|GetSeconds _returnvalue_5) _returnvalue)
      (Variables|Default|SetAs%20BP%20Save%20Leaderboard _returnvalue_5)
      (SaveGame|SaveGametoSlot _returnvalue_5 "GameSave")
      (Game|OpenLevel(byObjectReference) "/Game/ArtistFolder/Byron/Menu.Menu"))))

(fn Load
  (bind _returnvalue (SaveGame|DoesSaveGameExist "GameSave"))
  (if _returnvalue
    (bind _returnvalue_2 (SaveGame|LoadGamefromSlot "GameSave"))
    (bind _asbp_save_leaderboard (Utilities|Casting|CastToBP_SaveLeaderboard _returnvalue_2))
    (bind _output_get (Variables|Default|SetAs%20BP%20Save%20Leaderboard _asbp_save_leaderboard))
    (return (Variables|/Game/SpaceRaft/Blueprints/BP_SaveLeaderboard.BP_SaveLeaderboard_C|GetName _output_get) (Variables|/Game/SpaceRaft/Blueprints/BP_SaveLeaderboard.BP_SaveLeaderboard_C|GetMinutes _output_get) (Variables|/Game/SpaceRaft/Blueprints/BP_SaveLeaderboard.BP_SaveLeaderboard_C|GetSeconds _output_get))))